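; Interactable marker actor for an archviz project that runs an action set by its Action enum: opening a door, or a layout change whose handler is empty.
; It binds to the player's interact event, toggling the door by playing or reversing a level sequence.
; The construction script snaps it to the referenced door, sets status text and sphere radius.
; Overlaps and door interactions briefly flash custom-depth outlines.
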(event OnComponentBeginOverlap(Sphere_Collision)
  (params (OverlappedComponent :type Primitive%20Component%20Object%20Reference) (OtherActor :type Actor%20Object%20Reference) (OtherComp :type Primitive%20Component%20Object%20Reference) (OtherBodyIndex :type Integer) (bFromSweep :type Boolean) (SweepResult :type Hit%20Result%20Structure%20%28by%20ref%29))
  (bind _object_reference (Variables|01-Generic|GetObject%20Reference))
  (bind _staticmeshcomponent (Variables|/Script/Engine.StaticMeshActor|GetStaticMeshComponent _object_reference))
  (Rendering|SetRenderCustomDepth _staticmeshcomponent true)
  (Utilities|FlowControl|Delay 2.0)
  (Rendering|SetRenderCustomDepth _staticmeshcomponent false))

(event Custom|Interact
  (bind _open_door_seq (Variables|02-BpDoor|GetOpen%20door%20SEQ))
  (switch Utilities|FlowControl|Switch|SwitchonAction (Variables|01-Generic|GetAction)
    (:NewEnumerator0
      (Utilities|FlowControl|Sequence
        (:then_0
          (Utilities|FlowControl|Delay 0.5)
          (if (Variables|02-BpDoor|GetIsOpen)
            (bind _returnvalue (Sequencer|Player|CreateLevelSequencePlayer _open_door_seq))
            (Class|MovieSceneSequencePlayer|PlayReverse _returnvalue)
            (Variables|02-BpDoor|SetIsOpen false)
            (else
              (bind _returnvalue_2 (Sequencer|Player|CreateLevelSequencePlayer _open_door_seq))
              (Sequencer|Player|Play _returnvalue_2 :!class /Script/MovieScene.MovieSceneSequencePlayer)
              (Variables|02-BpDoor|SetIsOpen true))))
        (:then_1
          (Utilities|SetOutlineTimer))))
    (:NewEnumerator2
      (|LVS_Layout))))

(event EventBeginPlay
  (Utilities|FlowControl|Sequence
    (:then_0
      (bind _asbp_player_archvizz (Utilities|Casting|CastToBp_Player_Archvizz (Game|GetPlayerCharacter 0)))
      (Variables|Default|SetAs%20Bp%20AV%20Player _asbp_player_archvizz))
    (:then_1
      (bind _asbp_controller_archvizz (Utilities|Casting|CastToBp_Controller_Archvizz (Game|GetPlayerController 0)))
      (Variables|Default|SetAs%20Bp%20My%20Player%20Controller _asbp_controller_archvizz))
    (:then_2
      ;[0 0 0] E Event
      (EventDispatchers|BindEventtoInteract (Variables|Default|GetAs%20Bp%20AV%20Player) (delegate Custom|Interact)))))

(fn ConstructionScript
  (switch Utilities|FlowControl|Switch|SwitchonAction (Variables|01-Generic|GetAction)
    (:NewEnumerator0
      (|OpenDoor))))

(fn TextStatus
  (params (Value :type Text) (InLinearColor :type Linear%20Color%20Structure))
  (bind _textrender_02 (Variables|Default|GetTextRender_02))
  (Rendering|Components|TextRender|SetText _textrender_02 Value)
  (Rendering|Components|TextRender|SetTextRenderColor _textrender_02 (Class|KismetMathLibrary|LinearColortoRGBE InLinearColor))
  (return))

(fn HideMe
  (params (NewHidden :type Boolean))
  (Development|SetHiddeninGame (Variables|Default|GetTextRender_02) NewHidden true)
  (return))