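; Player character for an architectural visualization walkthrough, with mouse, touch and axis-driven movement, run and crouch.
; Dragging rotates the view, smoothed for the mouse and pitch-clamped for touch.
; A double click or tap traces from the screen point and, on FLOOR-tagged actors, auto-moves there and spawns a target marker.
; Teleporttolocation jumps to a target actor while a timeline eases control rotation; zoom autofocus logic exists but is unwired.
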(event Custom|Orient%20Character
  (params (Orient%20Rotation%20to%20Movement :type Boolean))
  (Variables|/Script/Engine.CharacterMovementComponent|SetbOrientRotationToMovement (Variables|Character|GetCharacterMovement) Orient%20Rotation%20to%20Movement))

(event Custom|Teleport%20to%20location
  (params (TargetLocation :type Actor%20Object%20Reference))
  ;[0 0 0] GO TO LOCATION
  (Variables|Default|SetLocation%20Target TargetLocation)
  (AI|Navigation|StopMovement (Variables|Default|GetAs%20Bp%20My%20Player%20Controller))
  (Utilities|FlowControl|Sequence
    (:then_0
      (Variables|Default|SetReturn%20Value%20Y%20%28Pitch%29_0 (.pitch (Transformation|GetWorldRotation (Variables|Default|GetCineCamera))))
      (Variables|Default|SetReturn%20Value%20Z%20%28Yaw%29 (.yaw (Pawn|GetControlRotation (Variables|Default|GetAs%20Bp%20My%20Player%20Controller) :!class /Script/Engine.Controller))))
    (:then_1
      (Transformation|Teleport (Transformation|GetActorLocation (Variables|Default|GetLocation%20Target)) (Transformation|GetActorRotation (Variables|Default|GetLocation%20Target))))
    (:then_2
      (bind _newtrack_0 (Timeline|Timeline_Location PlayFromStart)
        (:Update
          (Pawn|SetControlRotation (Variables|Default|GetAs%20Bp%20My%20Player%20Controller) (Math|Rotator|MakeRotator 0.0 (Math|Float|Lerp (Variables|Default|GetReturn%20Value%20Y%20%28Pitch%29_0) 0.0 _newtrack_0) (Math|Float|Lerp (Variables|Default|GetReturn%20Value%20Z%20%28Yaw%29) (.yaw (Transformation|GetActorRotation (Variables|Default|GetLocation%20Target))) _newtrack_0))))))))

(event EventBeginPlay
  (Utilities|FlowControl|Sequence
    (:then_0
      (bind _asbp_controller_archvizz (Utilities|Casting|CastToBp_Controller_Archvizz (Game|GetPlayerController 0)))
      (Variables|Default|SetAs%20Bp%20My%20Player%20Controller _asbp_controller_archvizz))
    (:then_1
      (Variables|/Script/CinematicCamera.CineCameraComponent|SetCurrentFocalLength (Variables|Default|GetCineCamera) (Variables|Default|GetFocal%20Lenght)))
    (:then_2)))

(event Input|AxisEvents|InputAxisMoveRight
  (params (AxisValue :type Float%20%28single-precision%29))
  (bind _speed (Variables|Default|Getspeed))
  (bind _returnvalue (* AxisValue _speed))
  ;[0 0 0] MOVEMENT
  (Pawn|Input|AddMovementInput (Transformation|GetActorRightVector) (Math|Float|SelectFloat (* _returnvalue 3.0) _returnvalue (Variables|Default|GetisRun)) false))

(event Input|AxisEvents|InputAxisMoveForward
  (params (AxisValue :type Float%20%28single-precision%29))
  (bind _speed (Variables|Default|Getspeed))
  (bind _returnvalue (* AxisValue _speed))
  ;[0 0 0] MOVEMENT
  (Pawn|Input|AddMovementInput (Transformation|GetActorForwardVector) (Math|Float|SelectFloat (* _returnvalue 3.0) _returnvalue (Variables|Default|GetisRun)) false))

(event Input|MouseEvents|MouseY
  (params (AxisValue :type Float%20%28single-precision%29))
  ;[0 0 0] PAN CHARACTER
  (if (Variables|Default|GetISCLICK)
    (bind _output_get (Variables|Default|SetCurrentYMouse (Math|Interpolation|FInterpTo (Variables|Default|GetCurrentYMouse) (* (* AxisValue (Variables|Default|GetMouseMultiply)) -1.0) (Utilities|Time|GetWorldDeltaSeconds) 1e+01)))
    (Pawn|Input|AddControllerPitchInput _output_get)))

(event Input|MouseEvents|MouseX
  (params (AxisValue :type Float%20%28single-precision%29))
  ;[0 0 0] PAN CHARACTER
  (if (Variables|Default|GetISCLICK)
    (bind _output_get (Variables|Default|SetCurrentXMouse (Math|Interpolation|FInterpTo (Variables|Default|GetCurrentXMouse) (* AxisValue (Variables|Default|GetMouseMultiply)) (Utilities|Time|GetWorldDeltaSeconds) 1e+01)))
    (Pawn|Input|AddControllerYawInput _output_get)))

(event Input|MouseEvents|RightMouseButton
  (params (Key :type Key%20Structure :default "None"))
  ;[0 0 0] ZOOM
)

(event Input|KeyboardEvents|LeftCtrl
  (params (Key :type Key%20Structure :default "None"))
  (bind _as_bp_my_player_controller (Variables|Default|GetAs%20Bp%20My%20Player%20Controller))
  (bind _canclick (Variables|/Game/Blueprint/Gamemode/Bp_Controller_Archvizz.Bp_Controller_Archvizz_C|GetCanClick _as_bp_my_player_controller))
  ;[0 0 0] CROUCH
  (:Pressed
    (if _canclick
      (Character|Crouch)))
  (:Released
    (if _canclick
      (Character|UnCrouch))))

(event Input|KeyboardEvents|LeftShift
  (params (Key :type Key%20Structure :default "None"))
  ;[0 0 0 0.5] Run
  (:Pressed
    (Variables|Default|SetisRun true))
  (:Released
    (Variables|Default|SetisRun false)))

(event Input|MouseEvents|LeftMouseButton
  (params (Key :type Key%20Structure :default "None"))
  (:Pressed
    (if (Variables|Default|GetISCLICK)
      (Variables|/Script/Engine.PlayerController|SetbShowMouseCursor (Game|GetPlayerController 0) true)
      (Variables|Default|SetIs_Tactil false)
      (Utilities|DoubleClick
        (:Double
          (bind (_location _is_floor) (CallFunction|GetClickTouchLocation))
          (if _is_floor
            (Utilities|FlowControl|Delay 0.2)
            (CallFunction|SimpleMoveLocation _location _is_floor)
            (else
              (Development|PrintString "NO TAG FLOOR"))))))))

(event Input|MouseEvents|LeftMouseButton
  (params (Key :type Key%20Structure :default "None"))
  (:Pressed
    (Variables|Default|SetISCLICK true))
  (:Released
    (Variables|Default|SetISCLICK false)))

(event Input|TouchEvents|InputTouch
  (params (Location :type Vector) (FingerIndex :type ETouchIndex%20Enum))
  (bind _returnvalue (Game|GetPlayerController 0))
  (bind (_locationx _locationy _biscurrentlypressed) (Class|PlayerController|GetInputTouchState _returnvalue "Touch1"))
  (:Pressed
    (if (Variables|Default|GetISCLICK)
      (Variables|Default|SetScreen%20Y (.y Location))
      (Variables|Default|SetScreen%20X (.x Location))
      (Utilities|FlowControl|Sequence
        (:then_0
          (Variables|/Script/Engine.PlayerController|SetbShowMouseCursor (Game|GetPlayerController 0) false)
          (Variables|Default|SetIs_Tactil true)
          (Utilities|DoubleClick
            (:Double
              (bind (_location _is_floor) (CallFunction|GetClickTouchLocation))
              (if _is_floor
                (Utilities|FlowControl|Delay 0.2)
                (CallFunction|SimpleMoveLocation _location _is_floor)
                (else
                  (Development|PrintString "NO TAG FLOOR"))))))
        (:then_1
          (Variables|Default|SetTouch_Hold true)
          (Variables|Default|SetTouch_Location_Previous (Math|Vector2D|MakeVector2D _locationx _locationy) :!label _label)))))
  (:Released
    (if true
      (Utilities|FlowControl|Sequence
        (:then_0
          (if (Variables|Default|GetTouch_Hold)
            (Variables|Default|SetTouch_Hold false)))
        (:then_1
          (goto _label)))))
  (:Moved
    (if true
      (Variables|Default|SetScreen%20Y (.y Location))
      (Variables|Default|SetScreen%20X (.x Location))
      (if _biscurrentlypressed
        (CallFunction|TouchRotation _locationx _locationy 75.0)))))

(fn ConstructionScript)

(fn GetClickTouchLocation
  (bind _returnvalue (Game|GetPlayerController 0))
  (bind _is_tactil (Variables|Default|GetIs_Tactil))
  (bind _screen_y (Variables|Default|GetScreen%20Y))
  (bind _screen_x (Variables|Default|GetScreen%20X))
  (bind (_worldlocation _worlddirection) (Game|Player|ConvertMouseLocationToWorldSpace _returnvalue))
  (bind (_worldlocation_2 _worlddirection_2) (Class|PlayerController|DeprojectScreenPositiontoWorld _returnvalue _screen_x _screen_y))
  (bind (_outhit _returnvalue_2) (Collision|LineTraceByChannel (Math|Vector|SelectVector _worldlocation_2 _worldlocation _is_tactil) (+ (Math|Vector|SelectVector _worldlocation_2 _worldlocation _is_tactil) (* (Math|Vector|SelectVector _worlddirection_2 _worlddirection _is_tactil) (Math|Conversions|ToVector(Float) 2.5e+03))) "TraceTypeQuery1" true 0 "ForDuration" true "(R=1.000000,G=0.000000,B=0.000000,A=1.000000)" "(R=0.000000,G=1.000000,B=0.000000,A=1.000000)" 2.0))
  (if _returnvalue_2
    (Variables|Default|SetHit%20Actor (.HitActor (Collision|BreakHitResult _outhit)))
    (return (.Location (Collision|BreakHitResult _outhit)) (Actor|ActorHasTag (.HitActor (Collision|BreakHitResult _outhit)) "FLOOR"))))

(fn SimpleMoveLocation
  (params (Location :type Vector) (Is%20Floor :type Boolean))
  (if Is%20Floor
    (AI|Navigation|SimpleMovetoLocation (Game|GetPlayerController 0) Location)
    (Game|SpawnActorfromClass "/Game/Blueprint/Character/Bp_TarguetPlayer.Bp_TarguetPlayer_C" (Math|Transform|MakeTransform Location "0, 0, 0" "1.000000,1.000000,1.000000") "Undefined" "OverrideRootScale" 0 0)
    (return)
    (else
      (Development|PrintString "NO FLOOR NAME"))))

(fn TouchRotation
  (params (Location_X :type Float%20%28double-precision%29) (Location_Y :type Float%20%28double-precision%29) (TouchRotation :type Float%20%28double-precision%29))
  (bind _returnvalue (Pawn|GetControlRotation :!class /Script/Engine.Pawn))
  (bind _returnvalue_2 (* TouchRotation -1.0))
  (Variables|Default|SetTouch_Location_Current (Math|Vector2D|MakeVector2D Location_X Location_Y))
  (Pawn|SetControlRotation (Game|GetPlayerController 0) (Math|Rotator|MakeRotator 0.0 (Math|Float|ClampAngle (+ (.pitch _returnvalue) (* (* (- (/ (.y (Variables|Default|GetTouch_Location_Current)) (.y (Variables|Default|GetTouch_Location_Previous))) 1.0) -1.0) _returnvalue_2)) (Variables|Default|GetPitchLimit_Min) (Variables|Default|GetPitchLimit_Max)) (+ (* (- (/ (.x (Variables|Default|GetTouch_Location_Current)) (.x (Variables|Default|GetTouch_Location_Previous))) 1.0) _returnvalue_2) (.yaw _returnvalue))))
  (Variables|Default|SetTouch_Location_Previous (Math|Vector2D|MakeVector2D (.x (Variables|Default|GetTouch_Location_Current)) (.y (Variables|Default|GetTouch_Location_Current)))))

(fn ViewDistance
  (bind _cinecamera (Variables|Default|GetCineCamera))
  (bind _returnvalue (Transformation|GetWorldLocation _cinecamera))
  (bind _outhit (Collision|LineTraceByChannel _returnvalue (+ _returnvalue (* (Math|Vector|GetForwardVector _cinecamera) (Math|Conversions|ToVector(Float) 5e+04))) "TraceTypeQuery1" true 0 "None" true "(R=1.000000,G=0.000000,B=0.000000,A=1.000000)" "(R=0.000000,G=1.000000,B=0.000000,A=1.000000)" 3.0))
  (Variables|/Script/CinematicCamera.CineCameraComponent|SetFocusSettings (Variables|Default|GetCineCamera) (Utilities|Struct|MakeCameraFocusSettings "Manual" (.Distance (Collision|BreakHitResult _outhit))))
  (return))

(fn GetDistancetoLocation
  (params (Destination :type Vector))
  (return (<= (Math|Vector|VectorLength (- Destination (Transformation|GetActorLocation))) 1e+02)))