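; Player controller for an architectural visualization game mode, handling session setup, level restart and floorplan view.
; On BeginPlay it runs performance-related console commands, caches player and game mode references, fades in from black, spawns the minimap and enables mouse input.
; An input action or RestartLevel01 event reloads the current level after a short delay.
; FloorplanObjects hides or shows ROOF-tagged static mesh actors by scanning all StaticMeshActors.
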(event Custom|RestartLevel01
  ;[0 0 0] RESTART LEVEL
  (Development|PrintString "Restart Level")
  (Utilities|FlowControl|Delay 1.0)
  (bind _returnvalue (Game|GetCurrentLevelName true))
  (Game|OpenLevel(byName) (Utilities|String|StringToName _returnvalue)))

(event EventBeginPlay
  (bind _returnvalue (Game|GetPlayerCameraManager 0))
  (Utilities|FlowControl|Sequence
    (:then_0
      (Development|ExecuteConsoleCommand "DumpUnbuiltLightInteractions" 0)
      (Development|ExecuteConsoleCommand "t.MaxFPS 5000" 0)
      (Development|ExecuteConsoleCommand "r.Streaming.PoolSize 20000" 0)
      (Development|ExecuteConsoleCommand "DisableAllScreenMessages" 0))
    (:then_1
      (bind _asbp_player_archvizz (Utilities|Casting|CastToBp_Player_Archvizz (Game|GetPlayerCharacter 0)))
      (Variables|Default|SetAs%20Bp%20AV%20Player _asbp_player_archvizz)
      (bind _asbp_gamemode_archvizz (Utilities|Casting|CastToBp_Gamemode_Archvizz (Game|GetGameMode)))
      (Variables|Default|SetAs%20Bp%20Gamemode%20Archvizz _asbp_gamemode_archvizz))
    (:then_3
      (Class|PlayerCameraManager|SetManualCameraFade :self _returnvalue :InFadeAmount 1.0 :bInFadeAudio true)
      (Utilities|FlowControl|Delay 1.0)
      (CameraFades|StartCameraFade :self _returnvalue :FromAlpha 1.0 :Duration 1.0 :bShouldFadeAudio true :bHoldWhenFinished true))
    (:then_5
      (Game|SpawnActorfromClass "/Game/Blueprint/Minimap/BP_Minimap.Bp_Minimap_C" (Math|Transform|MakeTransform "0, 0, 0") "Undefined" "MultiplyWithRoot" 0 0))
    (:then_6
      (Variables|Default|SetbShowMouseCursor true))
    (:then_7
      (Input|SetInputModeGameandUI self 0 "DoNotLock" true false))))

(event Input|ActionEvents|InputActionRestartLevel
  (params (Key :type Key%20Structure :default "None"))
  ;[0 0 0] RESTART LEVEL
  (:Pressed
    (Development|PrintString "Restart Level")
    (Utilities|FlowControl|Delay 1.0)
    (bind _returnvalue (Game|GetCurrentLevelName true))
    (Game|OpenLevel(byName) (Utilities|String|StringToName _returnvalue))))

(fn ConstructionScript)

(fn FloorplanObjects
  (params (bIsFloorplan :type Boolean))
  (if bIsFloorplan
    (Utilities|FlowControl|Sequence
      (:then_0
        (bind _outactors (Actor|GetAllActorsOfClass "/Script/Engine.StaticMeshActor"))
        (for _array_element _outactors
          (if (Actor|ActorHasTag _array_element "ROOF")
            (Rendering|SetActorHiddenInGame _array_element true))))
      (:then_1
        (return)))
    (else
      (Utilities|FlowControl|Sequence
        (:then_0
          (bind _outactors_2 (Actor|GetAllActorsOfClass "/Script/Engine.StaticMeshActor"))
          (for _array_element_2 _outactors_2
            (if (Actor|ActorHasTag _array_element_2 "ROOF")
              (Rendering|SetActorHiddenInGame _array_element_2 false))))
        (:then_1
          (return))))))